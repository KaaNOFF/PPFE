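; BP_Lava is a rising lava wall for a 2D game that kills the player character on contact.
; Each tick it moves up by WallSpeed, without delta-time scaling, then caps that speed at 0.75.
; Its box overlap calls PlayerDead once on the character cached at BeginPlay.
; The tile map is set in construction and again at BeginPlay, while a periodic speed-up block remains unconnected.
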(event `self.ReceiveTick`
  (params (DeltaSeconds :type "Float (single-precision)"))
  (`self.Up Height Wall`)
  (if (> (`self.Wall Speed`) 0.75)
    (set `self.Wall Speed` 0.75)))

(event `self.ReceiveBeginPlay`
  (bind _asbp_2d_character (cast `/Game/Blueprints/Player/BP_2dCharacter` (`GameplayStatics.GetPlayerCharacter` 0)))
  (set `self.As BP 2d Character` _asbp_2d_character)
  (`PaperTileMapComponent.SetTileMap` (`self.PaperTileMap`) (`self.New Tile Map`)))

(event `Up Height Wall`
  (bind (_returnvalue_x _returnvalue_y _returnvalue_z) (`KismetMathLibrary.BreakVector` (`self.K2_GetActorLocation`)))
  (`self.K2_SetActorLocation` (`KismetMathLibrary.MakeVector` _returnvalue_x _returnvalue_y (+ _returnvalue_z (`self.Wall Speed`)))))

(event `self.Box.OnComponentBeginOverlap`
  (params (OverlappedComponent :type "PrimitiveComponent Object Reference") (OtherActor :type "Actor Object Reference") (OtherComp :type "PrimitiveComponent Object Reference") (OtherBodyIndex :type Integer) (bFromSweep :type Boolean) (SweepResult :type "HitResult Structure (by ref)"))
  (if (== OtherActor (`GameplayStatics.GetPlayerCharacter` 0))
    (`/Engine/EditorBlueprintResources/StandardMacros.DoOnce` false
      (:`Completed`
        (`/Game/Blueprints/Player/BP_2dCharacter.Player Dead` (`self.As BP 2d Character`))))))

(fn `UserConstructionScript`
  (`PaperTileMapComponent.SetTileMap` (`self.PaperTileMap`) "/Game/TileMap/TM_Lava.TM_Lava"))