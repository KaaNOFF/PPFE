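; BP_Bullet_Crab is a projectile that deals damage on sphere overlap.
; On BeginPlay it reads LVLHeight from the player's BP_2dCharacter and scales Damage up in tiers as that value rises.
; Overlapping any actor without the MonsterPass tag applies that damage, spawns BP_Impact at the bullet's transform and destroys the bullet.
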(event `self.Sphere.OnComponentBeginOverlap`
  (params (OverlappedComponent :type "PrimitiveComponent Object Reference") (OtherActor :type "Actor Object Reference") (OtherComp :type "PrimitiveComponent Object Reference") (OtherBodyIndex :type Integer) (bFromSweep :type Boolean) (SweepResult :type "HitResult Structure (by ref)"))
  (if (not (`self.ActorHasTag` OtherActor "MonsterPass"))
    (`GameplayStatics.ApplyDamage` OtherActor (`self.Damage`))
    (`|SpawnActorFromClass` "/Game/Blueprints/Player/Bullet+FX/BP_Impact.BP_Impact_C" (`self.GetTransform`) "Undefined" "MultiplyWithRoot" null null)
    (`self.K2_DestroyActor`)))

(event `self.ReceiveBeginPlay`
  (bind _asbp_2d_character (cast `/Game/Blueprints/Player/BP_2dCharacter` (`GameplayStatics.GetPlayerCharacter` 0)))
  (bind _lvl_height (`/Game/Blueprints/Player/BP_2dCharacter.LVL Height` _asbp_2d_character))
  (if (>= _lvl_height 5)
    (set `self.Damage` 2.0)
    (if (>= _lvl_height 8)
      (set `self.Damage` 3.0)
      (if (>= _lvl_height 11)
        (set `self.Damage` 4.0)))
    (else
      (set `self.Damage` 1.0))))

(fn `UserConstructionScript`)