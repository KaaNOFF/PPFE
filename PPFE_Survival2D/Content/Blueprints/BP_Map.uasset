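; BP_Map is a 2D level segment that, unless IsSpawn is set, configures its tilemap and monsters on BeginPlay.
; The player character's LVLLastInt picks one of eight tilemaps with matching spawn-point positions, and LVLHeight sets difficulty.
; Difficulty selects how many points spawn a random Jumper or Crab, cascading downward, though a Crab at the second point skips the first.
; Player overlap destroys the Box component.
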(event `self.Box.OnComponentBeginOverlap`
  (params (OverlappedComponent :type "PrimitiveComponent Object Reference") (OtherActor :type "Actor Object Reference") (OtherComp :type "PrimitiveComponent Object Reference") (OtherBodyIndex :type Integer) (bFromSweep :type Boolean) (SweepResult :type "HitResult Structure (by ref)"))
  (if (== OtherActor (`GameplayStatics.GetPlayerCharacter` 0))
    (`ActorComponent.K2_DestroyComponent` (`self.Box`))))

(event `self.ReceiveBeginPlay`
  (bind _returnvalue (`SceneComponent.K2_GetComponentToWorld` (`self.Monster Spawn 3`)))
  (bind _returnvalue_2 (`SceneComponent.K2_GetComponentToWorld` (`self.Monster Spawn 1`)))
  (bind _returnvalue_3 (`SceneComponent.K2_GetComponentToWorld` (`self.Monster Spawn 2`)))
  (if (not (`self.Is Spawn`))
    (bind _asbp_2d_character (cast `/Game/Blueprints/Player/BP_2dCharacter` (`GameplayStatics.GetPlayerCharacter` 0))
      (:`then`
        (bind _lvl_height (`/Game/Blueprints/Player/BP_2dCharacter.LVL Height` _asbp_2d_character))
        ;[1 1 1] Set difficulty depending on LVL height
        (if (>= _lvl_height 2)
          (set `self.Difficulty` 1)
          (if (>= _lvl_height 4)
            (set `self.Difficulty` 2)
            (if (>= _lvl_height 6)
              (set `self.Difficulty` 3)))
          (else
            (set `self.Difficulty` 0)))
        ;[1 1 1] Randomly generate a tilemap and set scene in consequence for monster generation
        (switch `int` (`/Game/Blueprints/Player/BP_2dCharacter.LVL last int` _asbp_2d_character)
          (:`0`
            (set `self.Tile Map` "/Game/TileMap/TM_sandbox3.TM_sandbox3")
            (`SceneComponent.K2_SetRelativeLocation` (`self.Monster Spawn 1`) (400.0 0.0 -80.0) false false)
            (`SceneComponent.K2_SetRelativeLocation` (`self.Monster Spawn 2`) (701.0 0.0 -20.0) false false)
            (`SceneComponent.K2_SetRelativeLocation` (`self.Monster Spawn 3`) (175.0 0.0 -51.0) false false))
          (:`1`
            (set `self.Tile Map` "/Game/TileMap/TM_sandbox4.TM_sandbox4")
            (`SceneComponent.K2_SetRelativeLocation` (`self.Monster Spawn 1`) (360.0 0.0 -40.0) false false)
            (`SceneComponent.K2_SetRelativeLocation` (`self.Monster Spawn 2`) (295.0 0.0 -40.0) false false)
            (`SceneComponent.K2_SetRelativeLocation` (`self.Monster Spawn 3`) (480.0 0.0 -50.0) false false))
          (:`2`
            (set `self.Tile Map` "/Game/TileMap/TM_sandbox5.TM_sandbox5")
            (`SceneComponent.K2_SetRelativeLocation` (`self.Monster Spawn 1`) (135.0 0.0 -35.0) false false)
            (`SceneComponent.K2_SetRelativeLocation` (`self.Monster Spawn 2`) (710.0 0.0 -8.0) false false)
            (`SceneComponent.K2_SetRelativeLocation` (`self.Monster Spawn 3`) (408.0 0.0 -100.0) false false))
          (:`3`
            (set `self.Tile Map` "/Game/TileMap/TM_sandbox2_long.TM_sandbox2_long")
            (`SceneComponent.K2_SetRelativeLocation` (`self.Monster Spawn 1`) (455.0 0.0 -40.0) false false)
            (`SceneComponent.K2_SetRelativeLocation` (`self.Monster Spawn 2`) (168.0 0.0 -116.0) false false)
            (`SceneComponent.K2_SetRelativeLocation` (`self.Monster Spawn 3`) (265.0 0.0 -40.0) false false))
          (:`4`
            (set `self.Tile Map` "/Game/TileMap/TM_sandbox3_reverse.TM_sandbox3_reverse")
            (`SceneComponent.K2_SetRelativeLocation` (`self.Monster Spawn 1`) (400.0 0.0 -80.0) false false)
            (`SceneComponent.K2_SetRelativeLocation` (`self.Monster Spawn 2`) (100.0 0.0 -20.0) false false)
            (`SceneComponent.K2_SetRelativeLocation` (`self.Monster Spawn 3`) (625.0 0.0 -51.0) false false))
          (:`5`
            (set `self.Tile Map` "/Game/TileMap/TM_sandbox2_long_Reverse.TM_sandbox2_long_Reverse")
            (`SceneComponent.K2_SetRelativeLocation` (`self.Monster Spawn 1`) (540.0 0.0 -40.0) false false)
            (`SceneComponent.K2_SetRelativeLocation` (`self.Monster Spawn 2`) (186.0 0.0 -116.0) false false)
            (`SceneComponent.K2_SetRelativeLocation` (`self.Monster Spawn 3`) (350.0 0.0 -37.0) false false))
          (:`6`
            (set `self.Tile Map` "/Game/TileMap/TM_sandbox4_Reverse.TM_sandbox4_Reverse")
            (`SceneComponent.K2_SetRelativeLocation` (`self.Monster Spawn 1`) (440.0 0.0 -40.0) false false)
            (`SceneComponent.K2_SetRelativeLocation` (`self.Monster Spawn 2`) (520.0 0.0 -40.0) false false)
            (`SceneComponent.K2_SetRelativeLocation` (`self.Monster Spawn 3`) (320.0 0.0 -50.0) false false))
          (:`7`
            (set `self.Tile Map` "/Game/TileMap/TM_sandbox5_Reverse.TM_sandbox5_Reverse")
            (`SceneComponent.K2_SetRelativeLocation` (`self.Monster Spawn 1`) (690.0 0.0 -35.0) false false)
            (`SceneComponent.K2_SetRelativeLocation` (`self.Monster Spawn 2`) (180.0 0.0 -8.0) false false)
            (`SceneComponent.K2_SetRelativeLocation` (`self.Monster Spawn 3`) (390.0 0.0 -100.0) false false)))
        (`PaperTileMapComponent.SetTileMap` (`self.PaperTileMap`) (`self.Tile Map`))
        ;[1 1 1] Generate Monster
        (switch `int` (`self.Difficulty`)
          (:`1`
            (switch `int` (`KismetMathLibrary.RandomIntegerInRange` 0 1) :!label _label
              (:`0`
                (`|SpawnActorFromClass` "/Game/Blueprints/Enemy/BP_Jumper.BP_Jumper_C" _returnvalue_2 "AdjustIfPossibleButDontSpawnIfColliding" "MultiplyWithRoot" null null))
              (:`1`
                (`|SpawnActorFromClass` "/Game/Blueprints/Enemy/BP_Crab.BP_Crab_C" _returnvalue_2 "AdjustIfPossibleButDontSpawnIfColliding" "MultiplyWithRoot" null null))))
          (:`2`
            (switch `int` (`KismetMathLibrary.RandomIntegerInRange` 0 1) :!label _label_2
              (:`0`
                (`|SpawnActorFromClass` "/Game/Blueprints/Enemy/BP_Jumper.BP_Jumper_C" _returnvalue_3 "AdjustIfPossibleButDontSpawnIfColliding" "MultiplyWithRoot" null null)
                (goto _label))
              (:`1`
                (`|SpawnActorFromClass` "/Game/Blueprints/Enemy/BP_Crab.BP_Crab_C" _returnvalue_3 "AdjustIfPossibleButDontSpawnIfColliding" "MultiplyWithRoot" null null))))
          (:`3`
            (switch `int` (`KismetMathLibrary.RandomIntegerInRange` 0 1)
              (:`0`
                (`|SpawnActorFromClass` "/Game/Blueprints/Enemy/BP_Jumper.BP_Jumper_C" _returnvalue "AdjustIfPossibleButDontSpawnIfColliding" "MultiplyWithRoot" null null)
                (goto _label_2))
              (:`1`
                (`|SpawnActorFromClass` "/Game/Blueprints/Enemy/BP_Crab.BP_Crab_C" _returnvalue "AdjustIfPossibleButDontSpawnIfColliding" "MultiplyWithRoot" null null)
                (goto _label_2))))))
      (:`CastFailed`
        (`KismetSystemLibrary.PrintString` "Couldn't find player")))))

(fn `UserConstructionScript`
  (`PaperTileMapComponent.SetTileMap` (`self.PaperTileMap`) (`self.Tile Map`)))