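; BP_PowerUp is a pickup that targets the player's BP_2dCharacter.
; On BeginPlay it caches the player character, then compares it against any actor that overlaps its Sphere component.
; On a match it applies negative damage to the player, likely as healing, spawns BP_PowerUpEffect at the sprite's transform and destroys itself.
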(event `self.ReceiveBeginPlay`
  (bind _asbp_2d_character (cast `/Game/Blueprints/Player/BP_2dCharacter` (`GameplayStatics.GetPlayerCharacter` 0)))
  (set `self.Player ref` _asbp_2d_character))

(event `self.Sphere.OnComponentBeginOverlap`
  (params (OverlappedComponent :type "PrimitiveComponent Object Reference") (OtherActor :type "Actor Object Reference") (OtherComp :type "PrimitiveComponent Object Reference") (OtherBodyIndex :type Integer) (bFromSweep :type Boolean) (SweepResult :type "HitResult Structure (by ref)"))
  (bind _player_ref (`self.Player ref`))
  (if (== OtherActor _player_ref)
    (`GameplayStatics.ApplyDamage` _player_ref -1.0)
    (`|SpawnActorFromClass` "/Game/Blueprints/Player/Bullet+FX/BP_PowerUpEffect.BP_PowerUpEffect_C" (`SceneComponent.K2_GetComponentToWorld` (`self.Sprite`)) "Undefined" "MultiplyWithRoot" null null)
    (`self.K2_DestroyActor`)))

(fn `UserConstructionScript`)