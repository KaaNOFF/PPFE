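; Crab enemy for a 2D game that constantly walks along the X axis toward the player character, cached on BeginPlay.
; Each tick it adds movement input toward the player, rotates to face its travel direction, and switches between walk and idle flipbooks based on velocity.
; When standing still, the last chase direction decides its facing.
; Any damage destroys it immediately and spawns an impact actor in its place.
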(event `Handle Character Rotation`
  (bind _velocity_x (`KismetMathLibrary.BreakVector` (`MovementComponent.Velocity` (`self.CharacterMovement`))))
  (`/Engine/EditorBlueprintResources/StandardMacros.CompareFloat` _velocity_x
    (:`>`
      (`self.K2_SetActorRotation` (struct :`Yaw` 180.0) :!label _label))
    (:`==`
      (if (`self.Is moving Right ?`)
        (goto _label)
        (else
          (`self.K2_SetActorRotation` (struct) :!label _label_2))))
    (:`<`
      (goto _label_2))))

(event `self.ReceiveTick`
  (params (DeltaSeconds :type "Float (single-precision)"))
  (`self.Track Player`)
  (`self.Handle Character Rotation`)
  (`PaperFlipbookComponent.SetFlipbook` (`self.Sprite`) (select `bool` (> (`KismetMathLibrary.VSize` (`MovementComponent.Velocity` (`self.CharacterMovement`))) 0.0) :`false` "/Game/Assets/Ennemies/Crab/Idle/FB_crab-idle.FB_crab-idle" :`true` "/Game/Assets/Ennemies/Crab/Walk/FB_crab-walk.FB_crab-walk" :!type "PaperFlipbook Object Reference")))

(event `self.ReceiveBeginPlay`
  (bind _asbp_2d_character (cast `/Game/Blueprints/Player/BP_2dCharacter` (`GameplayStatics.GetPlayerCharacter` 0)))
  (set `self.Player Ref` _asbp_2d_character))

(event `Track Player`
  (bind _returnvalue_x (`KismetMathLibrary.BreakVector` (`self.K2_GetActorLocation`)))
  (bind _returnvalue_x_2 (`KismetMathLibrary.BreakVector` (`self.K2_GetActorLocation` (`self.Player Ref`))))
  (if (> _returnvalue_x_2 _returnvalue_x)
    (`PawnMovementComponent.AddInputVector` (`self.CharacterMovement`) (0.2 0.0 0.0) false)
    (set `self.Is moving Right ?` true)
    (else
      (`PawnMovementComponent.AddInputVector` (`self.CharacterMovement`) (-0.2 0.0 0.0) false)
      (set `self.Is moving Right ?` false))))

(event `self.ReceiveAnyDamage`
  (params (Damage :type "Float (single-precision)") (DamageType :type "DamageType Object Reference") (InstigatedBy :type "Controller Object Reference") (DamageCauser :type "Actor Object Reference"))
  (`|SpawnActorFromClass` "/Game/Blueprints/Player/Bullet/BP_ImpactEnnemy.BP_ImpactEnnemy_C" (`self.GetTransform`) "Undefined" "MultiplyWithRoot" null null)
  (`self.K2_DestroyActor`))

(fn `UserConstructionScript`)