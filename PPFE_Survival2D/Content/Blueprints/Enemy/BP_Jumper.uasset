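; BP_Jumper is a 2D enemy that hops toward the player along the X axis.
; A looping timer started at BeginPlay triggers each jump, and Tick keeps pushing movement input toward the player's side while it is airborne.
; Tick also swaps between jump and idle flipbooks based on whether it is falling.
; Any damage destroys it immediately, spawning an impact actor at its transform.
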(event `self.ReceiveBeginPlay`
  (bind _asbp_2d_character (cast `/Game/Blueprints/Player/BP_2dCharacter` (`GameplayStatics.GetPlayerCharacter` 0)))
  (set `self.Player Ref` _asbp_2d_character)
  (`KismetSystemLibrary.K2_SetTimerDelegate` (delegate `Jump to Player`) 1.5 true))

(event `Jump to Player`
  (bind _returnvalue_x (`KismetMathLibrary.BreakVector` (`self.K2_GetActorLocation`)))
  (bind _returnvalue_x_2 (`KismetMathLibrary.BreakVector` (`self.K2_GetActorLocation` (`self.Player Ref`))))
  (if (> _returnvalue_x_2 _returnvalue_x)
    (`PawnMovementComponent.AddInputVector` (`self.CharacterMovement`) (1.0 0.0 0.0) false)
    (`self.Jump`)
    (else
      (`PawnMovementComponent.AddInputVector` (`self.CharacterMovement`) (-1.0 0.0 0.0) false)
      (`self.Jump`))))

(event `self.ReceiveTick`
  (params (DeltaSeconds :type "Float (single-precision)"))
  (bind _sprite (`self.Sprite`))
  (`self.Move Direction`)
  (if (`NavMovementComponent.IsFalling` (`self.CharacterMovement`))
    (`PaperFlipbookComponent.SetFlipbook` _sprite "/Game/Assets/Ennemies/Jumper/Jump/FB_jumper-jump.FB_jumper-jump")
    (else
      (`PaperFlipbookComponent.SetFlipbook` _sprite "/Game/Assets/Ennemies/Jumper/Idle/FB_jumper-idle.FB_jumper-idle"))))

(event `Move Direction`
  (bind _returnvalue_x (`KismetMathLibrary.BreakVector` (`self.K2_GetActorLocation`)))
  (bind _returnvalue_x_2 (`KismetMathLibrary.BreakVector` (`self.K2_GetActorLocation` (`self.Player Ref`))))
  (if (`NavMovementComponent.IsFalling` (`self.CharacterMovement`))
    (if (> _returnvalue_x_2 _returnvalue_x)
      (`PawnMovementComponent.AddInputVector` (`self.CharacterMovement`) (1.0 0.0 0.0) false)
      (else
        (`PawnMovementComponent.AddInputVector` (`self.CharacterMovement`) (-1.0 0.0 0.0) false)))))

(event `self.ReceiveAnyDamage`
  (params (Damage :type "Float (single-precision)") (DamageType :type "DamageType Object Reference") (InstigatedBy :type "Controller Object Reference") (DamageCauser :type "Actor Object Reference"))
  (`|SpawnActorFromClass` "/Game/Blueprints/Player/Bullet/BP_ImpactEnnemy.BP_ImpactEnnemy_C" (`self.GetTransform`) "Undefined" "MultiplyWithRoot" null null)
  (`self.K2_DestroyActor`))

(fn `UserConstructionScript`)