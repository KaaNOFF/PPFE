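; Trampoline obstacle that launches the player character upward when it enters the box trigger.
; An overlap matching PlayerRef passes a DoOnce gate, applies a vertical launch with Z override and swaps the Paper2D sprite to the up state.
; After a reset delay, the sprite returns to the down state and ResetTrampoline reopens the gate for the next bounce.
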(event `self.Box.OnComponentBeginOverlap`
  (params (OverlappedComponent :type "PrimitiveComponent Object Reference") (OtherActor :type "Actor Object Reference") (OtherComp :type "PrimitiveComponent Object Reference") (OtherBodyIndex :type Integer) (bFromSweep :type Boolean) (SweepResult :type "HitResult Structure (by ref)"))
  (if (== OtherActor (`self.Player Ref`))
    (`/Engine/EditorBlueprintResources/StandardMacros.DoOnce` false :!label _label
      (:`Completed`
        (`Character.LaunchCharacter` (`self.Player Ref`) (`KismetMathLibrary.MakeVector` 0.0 0.0 (`self.Launch Velocity Z`)) false true)
        (`PaperSpriteComponent.SetSprite` (`self.PaperSprite`) "/Game/Assets/Level/Obstacles/Trampoline_Up.Trampoline_Up")
        (`KismetSystemLibrary.Delay` (`self.Reset Delay`))
        (`PaperSpriteComponent.SetSprite` (`self.PaperSprite`) "/Game/Assets/Level/Obstacles/Trampoline_Down.Trampoline_Down")
        (`self.Reset Trampoline`)))))

(event `Reset Trampoline`
  (goto _label :!via `Reset`))

(fn `UserConstructionScript`
  (`parent.UserConstructionScript`))