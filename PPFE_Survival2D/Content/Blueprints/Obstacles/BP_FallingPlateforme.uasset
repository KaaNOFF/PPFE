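; BP_FallingPlateforme is a sprite-based platform obstacle that drops after the player touches it.
; On the first player overlap with its Box, it waits DropDelay, then adds and activates a ProjectileMovement component and switches the sprite's collision object type to PhysicsBody.
; If Respawn is set, it spawns an actor at the saved starting location after RespawnDelay; otherwise it destroys itself after a fixed delay.
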(event `self.ReceiveBeginPlay`
  (`parent.ReceiveBeginPlay`)
  (set `self.Starting Location` (`self.K2_GetActorLocation`)))

(event `self.Box.OnComponentBeginOverlap`
  (params (OverlappedComponent :type "PrimitiveComponent Object Reference") (OtherActor :type "Actor Object Reference") (OtherComp :type "PrimitiveComponent Object Reference") (OtherBodyIndex :type Integer) (bFromSweep :type Boolean) (SweepResult :type "HitResult Structure (by ref)"))
  (if (== OtherActor (`self.Player Ref`))
    (`/Engine/EditorBlueprintResources/StandardMacros.DoOnce` false
      (:`Completed`
        (`KismetSystemLibrary.Delay` (`self.Drop Delay`))
        (bind _returnvalue (`AddComponent|NODE_AddProjectileMovementComponent-0` :`self` self))
        (`ActorComponent.SetActive` _returnvalue true false)
        (`PrimitiveComponent.SetCollisionObjectType` (`self.PaperSprite`) "ECC_PhysicsBody")
        (if (`self.Respawn ?`)
          (`KismetSystemLibrary.Delay` (`self.Respawn Delay`))
          (`|SpawnActorFromClass` "BP_FallingPlateforme_C" (`KismetMathLibrary.Conv_VectorToTransform` (`self.Starting Location`)) "Undefined" "MultiplyWithRoot" null 1.0 false null)
          (else
            (`KismetSystemLibrary.Delay` 6.0)
            (`self.K2_DestroyActor`)))))))

(fn `UserConstructionScript`
  (`parent.UserConstructionScript`))